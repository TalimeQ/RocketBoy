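; Bp_Chomik is an interactable dialogue actor that moves away once the player has a required item.
; On interaction, it searches the overlapping RocketBoy_BP's held items for item 2.
; Without it, it shows the default DialogBox text and calls the music dispatcher; with it, it shows alternate text and sets MoveChomiki.
; Tick then slides the actor along negative X at constant speed, unswept, until a fixed world limit.
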(event `self.ReceiveTick`
  (params (DeltaSeconds :type "Float (single-precision)"))
  (`parent.ReceiveTick` DeltaSeconds)
  (if (`self.bMoveChomiki`)
    (if (< -550.0 (.x (`self.K2_GetActorLocation`)))
      (`self.K2_AddActorWorldOffset` (`KismetMathLibrary.MakeVector` (* DeltaSeconds -15.0))))))

(event `self.Interacted`
  (bind _asrocket_boy_bp (cast `/Game/BP/RocketBoy_BP` (`|GetArrayItem` (`PrimitiveComponent.GetOverlappingActors` (`self.InteractZone`) "/Game/BP/RocketBoy_BP.RocketBoy_BP_C"))))
  (`/Engine/EditorBlueprintResources/StandardMacros.CompareInt` (`KismetArrayLibrary.Array_Find` (`/Game/BP/RocketBoy_BP.ItemzHeld` _asrocket_boy_bp) 2) -1
    (:`>`
      (bind _returnvalue (`|CreateWidget` "/Game/Widgets/DialogBox.DialogBox_C" (`GameplayStatics.GetPlayerController` 0) :!label _label))
      (set `/Game/Widgets/DialogBox.TextToDisplay` (`self.GoodTextTable`) _returnvalue)
      (set `/Game/Widgets/DialogBox.Order` (`self.Order2`) _returnvalue)
      (`UserWidget.AddToViewport` _returnvalue 0)
      (set `self.bMoveChomiki` true))
    (:`==`
      (bind _returnvalue_2 (`|CreateWidget` "/Game/Widgets/DialogBox.DialogBox_C" (`GameplayStatics.GetPlayerController` 0)))
      (set `/Game/Widgets/DialogBox.TextToDisplay` (`self.TextTable`) _returnvalue_2)
      (set `/Game/Widgets/DialogBox.Order` (`self.Integer`) _returnvalue_2)
      (`UserWidget.AddToViewport` _returnvalue_2 0)
      (`self.MusicDispatcher` 1))
    (:`<`
      (goto _label))))

(fn `UserConstructionScript`
  (`parent.UserConstructionScript`))