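; Bp_Marchew is a transient Paper2D flipbook actor for a carrot ("marchew") item that turns into its finished version.
; On BeginPlay it plays the flipbook without looping, waits a fixed short delay, spawns BP_MarchewFinished at its own location and rotation, then destroys itself.
; The swap is timer-driven; the OnFinishedPlaying binding to the Stop event is unconnected and never runs.
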(event `self.ReceiveBeginPlay`
  (`PaperFlipbookComponent.SetLooping` (`self.MarchewFlipbook`) false)
  (`parent.ReceiveBeginPlay`)
  (`KismetSystemLibrary.Delay` 1.5)
  (`|SpawnActorFromClass` "/Game/BP/Itemz/BP_MarchewFinished.BP_MarchewFinished_C" (`KismetMathLibrary.MakeTransform` (`self.K2_GetActorLocation`) (`self.K2_GetActorRotation`)) "Undefined" "OverrideRootScale" null null)
  (`self.K2_DestroyActor`))

(event `Stop`
  (`PaperFlipbookComponent.Stop` (`self.MarchewFlipbook`)))

(fn `UserConstructionScript`
  (`parent.UserConstructionScript`))