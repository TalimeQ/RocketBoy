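; BP_Plecak is an item pickup actor ("plecak" is Polish for backpack) that the RocketBoy_BP character collects into its inventory.
; On Interacted, it finds RocketBoy_BP actors overlapping InteractZone and calls AddToInventory with its item value, sprite and name, then destroys itself.
; ReturnSprite exposes the current sprite, while the BeginPlay, overlap and Tick events are disabled stubs.
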(event `self.Interacted`
  (for _array_element (`PrimitiveComponent.GetOverlappingActors` (`self.InteractZone`) "/Game/BP/RocketBoy_BP.RocketBoy_BP_C")
    (bind _asrocket_boy_bp (cast `/Game/BP/RocketBoy_BP` _array_element))
    (`/Game/BP/RocketBoy_BP.AddToInventory` _asrocket_boy_bp (`self.ItemValue`) (`PaperSpriteComponent.GetSprite` (`self.Sprite`)) (`self.ItemName`))
    (`self.K2_DestroyActor`)))

(fn `Return Sprite`
  (returns (NewParam :type "PaperSprite Object Reference"))
  (return (`PaperSpriteComponent.GetSprite` (`self.Sprite`))))

(fn `UserConstructionScript`
  (`parent.UserConstructionScript`))