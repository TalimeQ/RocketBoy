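; RocketBoy character Blueprint that moves a flipbook-animated sprite from player axis input.
; MoveForward and MoveRight share one chain that feeds Speed-scaled X/Y input into CharacterMovement.
; Nested axis-sign checks then select the Forward, Backward, Idle or GibuGibuNaBoki flipbook, rotating the sprite to mirror the latter.
; BeginPlay sets the camera boom's rotation and arm length.
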(event `InputAxis|MoveForward`
  (params (AxisValue :type "Float (single-precision)"))
  (bind _speed (`self.Speed`))
  (bind _rocketboyflipbook (`self.RocketBoyFlipBook`))
  (`PawnMovementComponent.AddInputVector` (`self.CharacterMovement`) (`KismetMathLibrary.MakeVector` (* AxisValue _speed) (* _speed (stale `InputAxis|MoveRight` AxisValue))) false :!label _label)
  (`/Engine/EditorBlueprintResources/StandardMacros.CompareFloat` AxisValue
    (:`>`
      (`PaperFlipbookComponent.SetFlipbook` (`self.RocketBoyFlipBook`) "/Game/Assets/GraphicalAssets/Sprites/Player/FlipBookz/Backward.Backward"))
    (:`==`
      (`/Engine/EditorBlueprintResources/StandardMacros.CompareFloat` (stale `InputAxis|MoveRight` AxisValue)
        (:`>`
          (`SceneComponent.K2_SetRelativeRotation` _rocketboyflipbook (struct :`Yaw` -90.0 :`Roll` 90.0) false false)
          (`PaperFlipbookComponent.SetFlipbook` (`self.RocketBoyFlipBook`) "/Game/Assets/GraphicalAssets/Sprites/Player/FlipBookz/GibuGibuNaBoki.GibuGibuNaBoki" :!label _label_2))
        (:`==`
          (`PaperFlipbookComponent.SetFlipbook` _rocketboyflipbook "/Game/Assets/GraphicalAssets/Sprites/Player/FlipBookz/Idle.Idle"))
        (:`<`
          (`SceneComponent.K2_SetRelativeRotation` _rocketboyflipbook (struct :`Pitch` 180.0 :`Yaw` -90.0 :`Roll` 90.0) false false)
          (goto _label_2))))
    (:`<`
      (`PaperFlipbookComponent.SetFlipbook` (`self.RocketBoyFlipBook`) "/Game/Assets/GraphicalAssets/Sprites/Player/FlipBookz/Forward.Forward"))))

(event `InputAxis|MoveRight`
  (params (AxisValue :type "Float (single-precision)"))
  (goto _label))

(event `self.ReceiveBeginPlay`
  (bind _cameraboom (`self.CameraBoom`))
  (`SceneComponent.K2_SetWorldLocationAndRotation` _cameraboom (0.0 0.0 0.0) (struct :`Pitch` -90.0) false false)
  (set `SpringArmComponent.TargetArmLength` 400.0 _cameraboom))

(fn `UserConstructionScript`)